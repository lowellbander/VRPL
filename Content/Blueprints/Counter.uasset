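; Counter is an actor that visualizes the item count of an assigned Collection through its own height.
; SetCollection stores the Collection reference that the actor reads from.
; Every Tick it polls GetCount and rebuilds its transform, keeping location and rotation while setting the Z scale to twice the count.
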(event `self.ReceiveBeginPlay`)

(event `self.ReceiveTick`
  (params (DeltaSeconds :type "Float (single-precision)"))
  (bind _count (`/Game/Blueprints/Collection.Get Count` (`self.Collection`)))
  (`self.K2_SetActorTransform` (`KismetMathLibrary.MakeTransform` (.location (`self.GetTransform`)) (.rotation (`self.GetTransform`)) (`KismetMathLibrary.MakeVector` 1.0 1.0 (`KismetMathLibrary.Conv_IntToDouble` (* _count 2))))))

(fn `Set Collection`
  (params (Collection :type "/Game/Blueprints/Collection Object Reference"))
  (set `self.Collection` Collection))

(fn `UserConstructionScript`)