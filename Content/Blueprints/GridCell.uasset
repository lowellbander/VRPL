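; GridCell is a clickable tile actor in a grid that stores its X/Y coordinates and can hold an entity.
; Clicking it looks up the Grid actor and asks it to hoist this cell by a fixed amount.
; Helpers set its altitude and compute its center from panel width, which TakeEntity uses to position the stored entity.
; GetCoordinates is a stub, and logic giving a CubeEntity to the origin cell is disconnected.
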(event `self.ReceiveBeginPlay`)

(event `self.ReceiveActorOnClicked`
  (params (ButtonPressed :type "Key Structure" :default "AnyKey"))
  (bind _outactors (`GameplayStatics.GetAllActorsOfClass` "/Game/Blueprints/Grid.Grid_C"))
  (`/Game/Blueprints/Grid.Hoist Cell` _outactors self 2000.0))

(fn `Get (X, Y)`
  (returns (X :type Integer) (Y :type Integer))
  (return (`self.X`) (`self.Y`)))

(fn `Get Center`
  (returns (Center :type "Vector Structure"))
  (bind _returnvalue (/ (`self.Panel Width`) 2.0))
  (return (+ (`self.K2_GetActorLocation`) (`KismetMathLibrary.MakeVector` _returnvalue _returnvalue))))

(fn `Get Coordinates`
  (returns (X :type Integer))
  (return 0))

(fn `Set (X, Y)`
  (params (X :type Integer) (Y :type Integer))
  (set `self.X` X)
  (set `self.Y` Y))

(fn `Set Altitude`
  (params (Altitude :type "Float (double-precision)"))
  (`self.K2_SetActorLocation` (`KismetMathLibrary.MakeVector` (.x (`self.K2_GetActorLocation`)) (.y (`self.K2_GetActorLocation`)) Altitude)))

(fn `Take Entity`
  (params (Entity :type "/Game/Blueprints/Entity Object Reference"))
  (bind _output_get (set `self.Entity` Entity))
  (bind _center (`self.Get Center`))
  (`self.K2_SetActorLocation` _output_get _center false false)
  (`KismetSystemLibrary.PrintString` "took entity"))

(fn `UserConstructionScript`)