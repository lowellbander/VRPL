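; Collection is an actor that holds and displays a set of Entities as a node feeding Filter actors.
; On BeginPlay it scales itself up and spawns a linked Counter above.
; It can fill itself from a selected Entity's four neighbors.
; Set destroys the old contents, spawns fresh actors of the given classes in a diagonal row, then updates every Filter whose Input is this Collection.
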(event EventBeginPlay
  (bind _returnvalue (Transformation|GetActorTransform))
  (bind (_location _rotation _scale) (Math|Transform|BreakTransform _returnvalue))
  (Transformation|SetActorTransform (Math|Transform|MakeTransform _location _rotation "10.000000,10.000000,10.000000"))
  (bind _returnvalue_2 (Game|SpawnActorfromClass "/Game/Blueprints/Counter.Counter_C" (Math|Transform|MakeTransform (+ _location "0, 0,1000.000000") _rotation _scale) "Undefined" 0 0))
  (Default|SetCollection _returnvalue_2 self))

(event Collision|EventActorBeginOverlap
  (params (OtherActor :type Actor%20Object%20Reference)))

(event EventTick
  (params (DeltaSeconds :type Float%20%28single-precision%29)))

(fn ConstructionScript)

(fn SetEntitiestoNeighborsOfSelection
  (params (Selected%20Entity :type Entity%20Object%20Reference))
  (bind _casted_entities (LocalVariables|GetCasted%20Entities))
  (bind (_bottom_neighbor _top_neighbor _left_neighbor _right_neighbor) (Default|GetNeighbors Selected%20Entity))
  (bind _filteredarray (Utilities|Array|FilterArray (Utilities|Array|MakeArray _bottom_neighbor _top_neighbor _left_neighbor _right_neighbor) "/Game/Blueprints/Entity.Entity_C"))
  (for _array_element _filteredarray
    (bind _asentity (Utilities|Casting|CastToEntity _array_element))
    (Utilities|Array|Add _casted_entities _asentity))
  (CallFunction|Set _casted_entities))

(fn Clear
  (bind _entities (Variables|Default|GetEntities))
  (for _array_element _entities
    (Actor|DestroyActor _array_element))
  (Utilities|Array|Clear _entities))

(fn Set
  (params (Entities :type Array%20of%20Entity%20Object%20References))
  (CallFunction|Clear)
  (for (_array_element _array_index) Entities
    (bind _returnvalue (Game|SpawnActorfromClass (Utilities|GetClass _array_element) (Math|Conversions|ToTransform(Vector) (+ (Transformation|GetActorLocation) (* (* "1.000000,1.000000,1.000000" _array_index) 75) "0,0,100.000000")) "Undefined" 0 0))
    (Utilities|Array|Add (Variables|Default|GetEntities) _returnvalue))
  (bind _outactors (Actor|GetAllActorsOfClass "/Game/Blueprints/Filter.Filter_C"))
  (for _array_element_2 _outactors
    (if (== (Variables|/Game/Blueprints/Filter.Filter_C|GetInput _array_element_2) self)
      (Default|Update _array_element_2))))

(fn GetCount
  (return (Utilities|Array|Length (Variables|Default|GetEntities))))