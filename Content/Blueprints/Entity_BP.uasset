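; Entity_BP is a grid entity actor that holds X and Y coordinates and has its position set through a Grid_BP.
; On BeginPlay it finds the single Grid_BP in the level, printing an error otherwise, and places itself with MoveGridEntity.
; Increment and decrement functions for X and Y change the coordinate, then call UpdateGridPosition to move it through the grid.
; Clicking the actor only prints a debug message.
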(event `self.ReceiveBeginPlay`
  (bind _outactors (`GameplayStatics.GetAllActorsOfClass` "/Game/Blueprints/Grid_BP.Grid_BP_C"))
  (if (!= (`KismetArrayLibrary.Array_Length` _outactors) 1)
    (`KismetSystemLibrary.PrintString` "Cone found too many or too few grids (there should be exactly one)")
    (else
      (set `self.Grid` (`KismetArrayLibrary.Array_Get` _outactors))
      (`/Game/Blueprints/Grid_BP.Move Grid Entity` (`self.Grid`) self (`self.X`) (`self.Y`)))))

(event `self.ReceiveActorOnClicked`
  (params (ButtonPressed :type "Key Structure" :default "AnyKey"))
  (`KismetSystemLibrary.PrintString` "clicked on Cone"))

(fn `Decrement X`
  (`/Engine/EditorBlueprintResources/StandardMacros.DecrementInt` (`self.X`)
    (:`  `
      (`self.Update Grid Position`))))

(fn `Decrement Y`
  (`/Engine/EditorBlueprintResources/StandardMacros.DecrementInt` (`self.Y`)
    (:`  `
      (`self.Update Grid Position`))))

(fn `Increment Y`
  (`/Engine/EditorBlueprintResources/StandardMacros.IncrementInt` (`self.Y`)
    (:`  `
      (`self.Update Grid Position`))))

(fn `IncrementX`
  (`/Engine/EditorBlueprintResources/StandardMacros.IncrementInt` (`self.X`)
    (:`  `
      (`self.Update Grid Position`))))

(fn `Update Grid Position`
  (`/Game/Blueprints/Grid_BP.Move Grid Entity` (`self.Grid`) self (`self.X`) (`self.Y`)))

(fn `UserConstructionScript`)