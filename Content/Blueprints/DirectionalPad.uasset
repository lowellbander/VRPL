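; Clickable directional pad actor that, when triggered, orders every Entity actor to move in the pad's current direction.
; Clicking cycles the direction through Right, Down, Left, Up and Random, yawing the pad in quarter turns to match.
; Entering or leaving Random rolls the pad half a turn to flip it over.
; OnTrigger looks up all Entity actors afresh and calls MoveInDirection on each.
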(event `self.ReceiveBeginPlay`
  (bind _outactors (`GameplayStatics.GetAllActorsOfClass` "/Game/Blueprints/Entity.Entity_C"))
  (set `self.Entity` (`KismetArrayLibrary.Array_Get` _outactors)))

(event `self.ReceiveActorOnClicked`
  (params (ButtonPressed :type "Key Structure" :default "AnyKey"))
  (`self.Rotate`))

(event `/Game/Blueprints/Triggerable.On Trigger`
  (bind _outactors (`GameplayStatics.GetAllActorsOfClass` "/Game/Blueprints/Entity.Entity_C"))
  (for _array_element _outactors
    (`/Game/Blueprints/Entity.Move In Direction` _array_element (`self.Direction`))))

(fn `Rotate`
  (switch `/Game/Blueprints/Direction` (`self.Direction`)
    (:`NewEnumerator0`
      (set `self.Direction` (cast `/Game/Blueprints/Direction` (+ (`self.Direction`) 1)) :!label _label)
      (`self.K2_SetActorRotation` (`KismetMathLibrary.MakeRotator` 0.0 0.0 (* (`KismetMathLibrary.Conv_ByteToInt` (`self.Direction`)) 90.0))))
    (:`NewEnumerator1`
      (goto _label))
    (:`NewEnumerator2`
      (goto _label))
    (:`NewEnumerator3`
      (set `self.Direction` (cast `/Game/Blueprints/Direction` (+ (`self.Direction`) 1)))
      (`self.K2_AddActorLocalRotation` (`KismetMathLibrary.MakeRotator` 180.0) :!label _label_2))
    (:`NewEnumerator4`
      (set `self.Direction` "NewEnumerator0")
      (goto _label_2))))

(fn `UserConstructionScript`)