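; Cone Blueprint that registers itself as an entity on the level's grid and responds to mouse clicks with a debug message.
; On BeginPlay it searches for Grid_BP actors, prints an error unless exactly one exists, and otherwise caches that grid and adds itself at the origin cell through AddEntityToGrid.
; The click handler only prints, and Tick and overlap events are unused.
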(event `self.ReceiveBeginPlay`
  (bind _outactors (`GameplayStatics.GetAllActorsOfClass` "/Game/Developer/Grid_BP.Grid_BP_C"))
  (if (!= (`KismetArrayLibrary.Array_Length` _outactors) 1)
    (`KismetSystemLibrary.PrintString` "Cone found too many or too few grids (there should be exactly one)")
    (else
      (set `self.Grid` (`KismetArrayLibrary.Array_Get` _outactors))
      (`/Game/Developer/Grid_BP.Add Entity to Grid` (`self.Grid`) self 0 0))))

(event `self.ReceiveActorOnClicked`
  (params (ButtonPressed :type "Key Structure" :default "AnyKey"))
  (`KismetSystemLibrary.PrintString` "clicked on Cone"))

(fn `UserConstructionScript`)