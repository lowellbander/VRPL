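; Grid actor that builds a flat X by Y floor of static mesh panels at BeginPlay and places entities on it.
; ConstructGrid loops over rows and AddXPanels adds a mesh component per cell, spaced by panel width plus gap.
; AddEntityToGrid range-checks a cell's upper bounds, then moves the passed actor above it.
; That target offsets the cell corner by a full PanelWidth and is set as a world location, ignoring the grid's transform.
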(event `self.ReceiveBeginPlay`
  (`self.Construct Grid`))

(fn `(X, Y) to Panel Center`
  (params (X :type Integer) (Y :type Integer) (`Z Offset` :type "Float (double-precision)"))
  (returns (Center :type "Vector Structure"))
  (bind _panel_width (`self.panel width`))
  (bind _position (`self.Convert Index to Panel Corner` X))
  (bind _position_2 (`self.Convert Index to Panel Corner` Y))
  (return (`KismetMathLibrary.MakeVector` (+ _position _panel_width) (+ _position_2 _panel_width) `Z Offset`)))

(fn `Add Entity to Grid`
  (params (Cone :type "/Game/Developer/Cone_BP Object Reference") (X :type Integer) (Y :type Integer))
  (`KismetSystemLibrary.PrintString` "Adding Entity to Grid")
  (if (and (< X (`self.# of X Panels`)) (< Y (`self.# of Y Panels`)))
    (bind _center (`self.(X, Y) to Panel Center` X Y 150.0))
    (`self.K2_SetActorLocation` Cone _center false false)
    (else
      ;[1 1 1] Error Handling
      (`KismetSystemLibrary.PrintString` "can't place entity out of grid range"))))

(fn `Add X Panels`
  (params (`Y Offset` :type "Float (double-precision)"))
  (for _index (range (+ (`self.# of X Panels`) 1))
    (bind _position (`self.Convert Index to Panel Corner` _index))
    (`AddComponent|StaticMeshComponent_0` :`RelativeTransform` (`KismetMathLibrary.Conv_VectorToTransform` (`KismetMathLibrary.MakeVector` _position `Y Offset`)))))

(fn `addYPanels`)

(fn `Construct Grid`
  (`KismetSystemLibrary.PrintString` "construct grid")
  (for _index (range (+ (`self.# of Y Panels`) 1))
    (bind _position (`self.Convert Index to Panel Corner` _index))
    (`self.Add X Panels` _position)))

(fn `Convert Index to Panel Corner`
  (params (Index :type Integer))
  (returns (Position :type "Float (double-precision)"))
  (return (* Index (+ (`self.Gap Width`) (`self.panel width`)))))

(fn `Print Vector`
  (params (`Input Vector` :type "Vector Structure"))
  (`KismetSystemLibrary.PrintString` "Vector:")
  (`KismetSystemLibrary.PrintText` (`|FormatText` "X: {x}" (`KismetTextLibrary.Conv_DoubleToText` (.x `Input Vector`) "HalfToEven")))
  (`KismetSystemLibrary.PrintText` (`|FormatText` "Y: {x}" (`KismetTextLibrary.Conv_DoubleToText` (.y `Input Vector`) "HalfToEven")))
  (`KismetSystemLibrary.PrintText` (`|FormatText` "Z: {x}" (`KismetTextLibrary.Conv_DoubleToText` (.z `Input Vector`) "HalfToEven"))))

(fn `UserConstructionScript`
  (`KismetSystemLibrary.PrintString` "Hello"))